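; BP_Sphere is a sphere actor that relocates when a BP_Agent touches it, apparently a target for the agents in the Backpropagation project.
; Its collision component's begin-overlap event ignores any actor that is not a BP_Agent.
; On a valid overlap, it jumps to a uniformly random X and Y within 1000 units of the world origin on each axis, keeping its current height.
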(event `self.SphereCollision.OnComponentBeginOverlap`
  (params (OverlappedComponent :type "PrimitiveComponent Object Reference") (OtherActor :type "Actor Object Reference") (OtherComp :type "PrimitiveComponent Object Reference") (OtherBodyIndex :type Integer) (bFromSweep :type Boolean) (SweepResult :type "HitResult Structure (by ref)"))
  (bind (_returnvalue_x _returnvalue_y _returnvalue_z) (`KismetMathLibrary.BreakVector` (`self.K2_GetActorLocation`)))
  (cast `/Game/Blueprints/Backpropagation/BP_Agent` OtherActor)
  (`self.K2_SetActorLocation` (`KismetMathLibrary.MakeVector` (* (- (* (`KismetMathLibrary.RandomFloat`) 2.0) 1.0) 1000.0) (* (- (* (`KismetMathLibrary.RandomFloat`) 2.0) 1.0) 1000.0) _returnvalue_z)))

(fn `UserConstructionScript`)