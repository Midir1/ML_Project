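; BP_RLTrainingManager drives reinforcement learning training of a driving agent through the Learning Agents plugin.
; On BeginPlay it sets up the interactor, builds the policy on that interactor and the DA_DrivingNetwork asset, then gives both to the RL trainer.
; Each Tick calls RunTraining with trainer, game, path and critic settings, without reinitializing the policy network.
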(event `self.ReceiveBeginPlay`
  (bind _bp_drivingpolicy (`self.BP_DrivingPolicy`))
  (bind _bp_drivinginteractor (`self.BP_DrivingInteractor`))
  (`|ExecutionSequence`
    (:`then_0`
      (`LearningAgentsInteractor.SetupInteractor` _bp_drivinginteractor))
    (:`then_1`
      (`LearningAgentsPolicy.SetupPolicy` _bp_drivingpolicy _bp_drivinginteractor (`self.Policy Settings`) "/Game/DA_DrivingNetwork.DA_DrivingNetwork"))
    (:`then_2`
      (`LearningAgentsTrainer.SetupTrainer` (`self.BP_DrivingRLTrainer`) _bp_drivinginteractor _bp_drivingpolicy null (`self.Trainer Settings`)))))

(event `self.ReceiveTick`
  (params (DeltaSeconds :type "Float (single-precision)"))
  (`LearningAgentsTrainer.RunTraining` (`self.BP_DrivingRLTrainer`) (`self.Trainer Training Settings`) (`self.Trainer Game Settings`) (`self.Trainer Path Settings`) (`self.Critic Settings`) false true true))

(fn `UserConstructionScript`)